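; A random coin pickup that gambles with the player's currency when something overlaps it.
; On overlap it plays an explosion sound, then makes a 50/50 roll to add either its Currency or its Negativecurrency value to the GeffPlaceholder player pawn's Currency.
; It destroys itself after either outcome.
; The overlapping actor is not checked, so the change always targets player pawn 0.
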(event EventBeginPlay)

(event Collision|EventActorBeginOverlap
  (params (OtherActor :type Actor%20Object%20Reference))
  (Audio|PlaySound2D "/Game/StarterContent/Audio/Explosion01.Explosion01" 1.0 1.0 0.0 0 0)
  (if (== (Math|Random|RandomIntegerinRange 0 1) 0)
    (bind _asgeff_placeholder (Utilities|Casting|CastToGeffPlaceholder (Game|Player|GetPlayerPawn 0)))
    (Variables|/Game/Blueprints/GeffPlaceholder/GeffPlaceholder.GeffPlaceholder_C|SetCurrency _asgeff_placeholder (+ (Variables|/Game/Blueprints/GeffPlaceholder/GeffPlaceholder.GeffPlaceholder_C|GetCurrency _asgeff_placeholder) (Variables|Default|Getcurrency)))
    (Actor|DestroyActor)
    (else
      (bind _asgeff_placeholder_2 (Utilities|Casting|CastToGeffPlaceholder (Game|Player|GetPlayerPawn 0)))
      (Variables|/Game/Blueprints/GeffPlaceholder/GeffPlaceholder.GeffPlaceholder_C|SetCurrency _asgeff_placeholder_2 (+ (Variables|/Game/Blueprints/GeffPlaceholder/GeffPlaceholder.GeffPlaceholder_C|GetCurrency _asgeff_placeholder_2) (Variables|Default|Getnegativecurrency)))
      (Actor|DestroyActor))))

(fn ConstructionScript)