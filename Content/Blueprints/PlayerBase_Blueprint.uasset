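; PlayerBase Blueprint is the player's base, which tracks health and triggers game over when it runs out.
; On BeginPlay it caches the PlayerBaseHealth widget from its HealthBar component and sets current health to maximum.
; AnyDamage subtracts incoming damage and creates a GAMEOVER widget at zero or below, with no viewport add in this graph.
; The cached bar reference is not updated here.
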(event EventBeginPlay
  (bind _asplayer_base_health (Utilities|Casting|CastToPlayerBaseHealth (UserInterface|GetUserWidgetObject (Variables|Default|GetHealthBar))))
  (Variables|Default|SetBar _asplayer_base_health)
  ;[1 1 1] Setting Health of Player Base
  (Variables|Default|SetCurrentHealth (Variables|Default|GetMaxHealth)))

(event Game|Damage|EventAnyDamage
  (params (Damage :type Float%20%28single-precision%29) (DamageType :type Damage%20Type%20Object%20Reference) (InstigatedBy :type Controller%20Object%20Reference) (DamageCauser :type Actor%20Object%20Reference))
  ;[1 1 1] PlayerBase Damage Taken and Game Over Condition
  (Variables|Default|SetCurrentHealth (- (Variables|Default|GetCurrentHealth) Damage))
  (if (<= (Variables|Default|GetCurrentHealth) 0.0)
    (UserInterface|CreateWidget "/Game/Blueprints/GAMEOVER.GAMEOVER_C")))

(fn ConstructionScript)