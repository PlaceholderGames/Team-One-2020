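; Homing projectile, apparently for a tower, that chases a Target actor and damages it on contact.
; Each tick it moves toward the target at constant Speed, caching the target's last known location.
; Its sphere overlap applies Damage only to that target, then destroys the projectile.
; If the target becomes invalid, it flies on to the cached location and self-destructs; an explosion sound node is left unconnected.
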(event OnComponentBeginOverlap(Sphere)
  (params (OverlappedComponent :type Primitive%20Component%20Object%20Reference) (OtherActor :type Actor%20Object%20Reference) (OtherComp :type Primitive%20Component%20Object%20Reference) (OtherBodyIndex :type Integer) (bFromSweep :type Boolean) (SweepResult :type Hit%20Result%20Structure%20%28by%20ref%29))
  (bind _target (Variables|Default|GetTarget))
  (if (== OtherActor _target)
    (Game|Damage|ApplyDamage _target (Variables|Default|GetDamage) 0 0)
    (Actor|DestroyActor)))

(event EventBeginPlay)

(event Collision|EventActorBeginOverlap
  (params (OtherActor :type Actor%20Object%20Reference)))

(event EventTick
  (params (DeltaSeconds :type Float%20%28single-precision%29))
  (bind _target (Variables|Default|GetTarget))
  (bind _returnvalue (Transformation|GetActorLocation _target))
  (Utilities|IsValid _target
    (:Is%20Valid
      (Variables|Default|SetlastKnown _returnvalue)
      (Transformation|SetActorLocation (Math|Interpolation|VInterptoConstant (Transformation|GetActorLocation) _returnvalue DeltaSeconds (Variables|Default|GetSpeed)) false false))
    (:Is%20Not%20Valid
      (Transformation|SetActorLocation (Math|Interpolation|VInterptoConstant (Transformation|GetActorLocation) (Variables|Default|GetlastKnown) DeltaSeconds (Variables|Default|GetSpeed)) false false)
      (if (Math|Vector|Equal(Vector) (Transformation|GetActorLocation) (Variables|Default|GetlastKnown) 0.0001)
        (Actor|DestroyActor)))))

(fn ConstructionScript)