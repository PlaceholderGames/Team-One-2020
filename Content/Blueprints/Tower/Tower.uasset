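; Tower actor that automatically shoots Enemy actors within range, with mesh, range, muzzle height, damage and fire rate taken from NewTowerStruct.
; TargetArea overlaps set or clear the target.
; Without a target, Tick runs a throttled sphere trace for pawns and picks the closest Enemy.
; With one, it spawns projectiles carrying target and damage, using a Delay-reset reload flag to pace shots.
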(event OnComponentBeginOverlap(TargetArea)
  (params (OverlappedComponent :type Primitive%20Component%20Object%20Reference) (OtherActor :type Actor%20Object%20Reference) (OtherComp :type Primitive%20Component%20Object%20Reference) (OtherBodyIndex :type Integer) (bFromSweep :type Boolean) (SweepResult :type Hit%20Result%20Structure%20%28by%20ref%29))
  (Utilities|IsValid (Variables|Default|GettowerTarget)
    (:Is%20Not%20Valid
      (bind _asenemy (Utilities|Casting|CastToEnemy OtherActor))
      (Variables|Default|SettowerTarget _asenemy))))

(event OnComponentEndOverlap(TargetArea)
  (params (OverlappedComponent :type Primitive%20Component%20Object%20Reference) (OtherActor :type Actor%20Object%20Reference) (OtherComp :type Primitive%20Component%20Object%20Reference) (OtherBodyIndex :type Integer))
  (if (== OtherActor (Variables|Default|GettowerTarget))
    (Variables|Default|SettowerTarget 0)))

(event Custom|TowerInit
  (bind _newtowerstruct (Variables|Default|GetnewTowerStruct))
  (bind (_type _damage _range _firerate _projectilespeed _mesh _shootingheight) (Utilities|Struct|BreakNewTowerStruct _newtowerstruct))
  (bind _returnvalue (* "1.000000,1.000000,1.000000" _range))
  (Components|StaticMesh|SetStaticMesh (Variables|Default|GetTowerMesh) _mesh)
  (Transformation|SetRelativeScale3D (Variables|Default|GetTargetCircle) _returnvalue)
  (Transformation|SetRelativeScale3D (Variables|Default|GetTargetArea) _returnvalue)
  (Transformation|SetWorldLocation (Variables|Default|GetShooting%20Location) (+ (Transformation|GetWorldLocation (Variables|Default|GetTowerMesh)) _shootingheight) false false))

(event Custom|Fire
  (Audio|PlaySoundatLocation "/Game/Sounds/NoiseForFun/NFF-bubble-input.NFF-bubble-input" (Transformation|GetActorLocation) "0, 0, 0" 1.0 1.0 0.0 0 0 0)
  (Variables|Default|SetisReloading true)
  (Game|SpawnActorfromClass "/Game/Blueprints/Tower/NEWTowerProjectile.NEWTowerProjectile_C" (Math|Conversions|ToTransform(Vector) (Transformation|GetWorldLocation (Variables|Default|GetShooting%20Location))) "AlwaysSpawn" 0 (Variables|Default|GettowerTarget) (.Damage (Utilities|Struct|BreakNewTowerStruct (Variables|Default|GetnewTowerStruct))) 0)
  (Utilities|FlowControl|Delay (.FireRate (Utilities|Struct|BreakNewTowerStruct (Variables|Default|GetnewTowerStruct))))
  (Variables|Default|SetisReloading false))

(event Custom|CheckForNewTarget
  (bind _returnvalue (Transformation|GetActorLocation))
  (Variables|Default|SetisCheckingForTarget true)
  (bind (_outhits _returnvalue_2) (Collision|MultiSphereTraceForObjects _returnvalue (- _returnvalue "0, 0,1.000000") (.Range (Utilities|Struct|BreakNewTowerStruct (Variables|Default|GetnewTowerStruct))) (Utilities|Array|MakeArray "ObjectTypeQuery3") false 0 "None"))
  (if _returnvalue_2
    (bind _newtarget (CallFunction|ClosestTargetCalc _outhits))
    (Utilities|IsValid _newtarget
      (:Is%20Valid
        (Variables|Default|SettowerTarget _newtarget))
      (:Is%20Not%20Valid
        _)))
  (Utilities|FlowControl|Delay 0.2)
  (Variables|Default|SetisCheckingForTarget false))

(event EventBeginPlay
  (CallFunction|TowerInit))

(event EventTick
  (params (DeltaSeconds :type Float%20%28single-precision%29))
  (Utilities|IsValid (Variables|Default|GettowerTarget)
    (:Is%20Valid
      (if (not (Variables|Default|GetisReloading))
        (CallFunction|Fire)))
    (:Is%20Not%20Valid
      (if (not (Variables|Default|GetisCheckingForTarget))
        (CallFunction|CheckforNewTarget)))))

(fn ConstructionScript)

(fn ClosestTargetCalc
  (params (HitResults :type Array%20of%20Hit%20Result%20Structures))
  (for _array_element HitResults
    (bind _asenemy (Utilities|Casting|CastToEnemy (.HitActor (Collision|BreakHitResult _array_element))))
    (Utilities|IsValid (LocalVariables|GetTempTarget)
      (:Is%20Valid
        (if (< (Math|Vector|VectorLength (- (Transformation|GetActorLocation) (Transformation|GetActorLocation (.HitActor (Collision|BreakHitResult _array_element))))) (LocalVariables|GetTempDistance))
          (LocalVariables|SetTempTarget _asenemy)
          (LocalVariables|SetTempDistance (Math|Vector|VectorLength (- (Transformation|GetActorLocation) (Transformation|GetActorLocation (.HitActor (Collision|BreakHitResult _array_element))))))))
      (:Is%20Not%20Valid
        (LocalVariables|SetTempTarget _asenemy)
        (LocalVariables|SetTempDistance (Math|Vector|VectorLength (- (Transformation|GetActorLocation) (Transformation|GetActorLocation (.HitActor (Collision|BreakHitResult _array_element)))))))))
  (return (LocalVariables|GetTempTarget)))