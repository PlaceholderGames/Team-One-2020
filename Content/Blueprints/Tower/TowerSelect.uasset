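; TowerSelect is a tower actor, apparently for selection, that shows a tower's mesh and range.
; On BeginPlay it reads the "Basic" row of NewTowerData to set the mesh, scale a plane from Range and offset the shooting location above or from the mesh by ShootingHeight.
; A ClosestTargetCalc helper returns the nearest Enemy from hit results by distance, but nothing in this file calls it.
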(event EventBeginPlay
  (bind _self self)
  (bind _towermesh (Variables|TowerSelect_C|GetTowerMesh _self))
  (bind _returnvalue (Utilities|GetDataTableRow "/Game/Blueprints/Tower/NewTowerData.NewTowerData" "Basic")
    (:then
      (Components|StaticMesh|SetStaticMesh _towermesh (.Mesh (Utilities|Struct|BreakNewTowerStruct _returnvalue)))
      (Transformation|SetRelativeScale3D (Variables|TowerSelect_C|GetPlane _self) (Math|Vector|MakeVector (/ (.Range (Utilities|Struct|BreakNewTowerStruct _returnvalue)) 5e+01) (/ (.Range (Utilities|Struct|BreakNewTowerStruct _returnvalue)) 5e+01) 1.0))
      (Transformation|SetWorldLocation (Variables|TowerSelect_C|GetShooting%20Location _self) (+ (Transformation|GetWorldLocation _towermesh) (.ShootingHeight (Utilities|Struct|BreakNewTowerStruct _returnvalue))) false false))))

(event EventTick
  (params (DeltaSeconds :type Float%20%28single-precision%29)))

(fn ConstructionScript)

(fn ClosestTargetCalc
  (params (HitResults :type Array%20of%20Hit%20Result%20Structures))
  (for _array_element HitResults
    (bind _asenemy (Utilities|Casting|CastToEnemy (.HitActor (Collision|BreakHitResult _array_element))))
    (Utilities|IsValid (LocalVariables|GetTempTarget)
      (:Is%20Valid
        (if (< (Math|Vector|VectorLength (- (Transformation|GetActorLocation) (Transformation|GetActorLocation (.HitActor (Collision|BreakHitResult _array_element))))) (LocalVariables|GetTempDistance))
          (LocalVariables|SetTempTarget _asenemy)
          (LocalVariables|SetTempDistance (Math|Vector|VectorLength (- (Transformation|GetActorLocation) (Transformation|GetActorLocation (.HitActor (Collision|BreakHitResult _array_element))))))))
      (:Is%20Not%20Valid
        (LocalVariables|SetTempTarget _asenemy)
        (LocalVariables|SetTempDistance (Math|Vector|VectorLength (- (Transformation|GetActorLocation) (Transformation|GetActorLocation (.HitActor (Collision|BreakHitResult _array_element)))))))))
  (return (LocalVariables|GetTempTarget)))