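; Wave spawner actor that runs five enemy waves and shows a win screen once they are cleared.
; Every tick it prints debug values and recounts Enemy actors; at zero, it sets the current wave's counts and calls StartWave.
; StartWave spawns Normal, Fast and Strong groups as AI pawns at random points inside the SpawnArea bounds, with short delays between groups, then advances the wave.
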(event Custom|StartWave
  (bind _wcurrent (Variables|Default|GetwCurrent))
  (bind (_normal _fast _strong) (Utilities|Struct|Breakwave _wcurrent))
  (bind (_number _type) (Utilities|Struct|BreakenemyInfo _normal))
  (bind (_number_2 _type_2) (Utilities|Struct|BreakenemyInfo _fast))
  (bind (_number_3 _type_3) (Utilities|Struct|BreakenemyInfo _strong))
  ;[1 1 1] For WCurrent thing
  (for _index (range 0 0)
    (for _index_2 (range 1 _number)
      (CallFunction|SpawnEnemy _type))
    (Utilities|FlowControl|Delay 0.5)
    (for _index_3 (range 1 _number_2)
      (CallFunction|SpawnEnemy _type_2))
    (Utilities|FlowControl|Delay 0.5)
    (for _index_4 (range 1 _number_3)
      (CallFunction|SpawnEnemy _type_3))
    (Math|Integer|IncrementInt (Variables|Default|GetWave))))

(event Custom|SpawnEnemy
  (params (currentEnemy :type Pawn%20Class%20Reference))
  (bind _spawnarea (Variables|Default|GetSpawnArea))
  (bind _boxextent (Collision|GetComponentBounds _spawnarea))
  ;[1 1 1] Wave Spawning Areas
  (AI|SpawnAIFromClass currentEnemy 0 (+ (Math|Vector|MakeVector (Math|Random|RandomFloatinRange (* (.x _boxextent) -1.0) (.x _boxextent)) (Math|Random|RandomFloatinRange (* (.y _boxextent) -1.0) (.y _boxextent)) (Math|Random|RandomFloatinRange (* (.z _boxextent) -1.0) (.z _boxextent))) (Transformation|GetWorldLocation _spawnarea)) "0, 0, 0" false)
  (Math|Integer|IncrementInt (Variables|Default|GetEnemiesLeft)))

(event EventTick
  (params (DeltaSeconds :type Float%20%28single-precision%29))
  ;[1 1 1] Starting Wave
  (Development|PrintString (Utilities|String|ToString(Integer) (Variables|Default|GetWave)))
  (Development|PrintString (Utilities|String|ToString(Integer) (Variables|Default|GetEnemiesLeft)))
  (Variables|Default|SetEnemiesLeft 0)
  (bind _outactors (Actor|GetAllActorsOfClass "/Game/Blueprints/Enemies/Enemy.Enemy_C"))
  (for _array_element _outactors
    (Math|Integer|IncrementInt (Variables|Default|GetEnemiesLeft)))
  (if (not (Math|Conversions|ToBoolean(Integer) (Variables|Default|GetEnemiesLeft)))
    (switch int (Variables|Default|GetWave)
      (:0
        (CallFunction|SetWaveInfo 1)
        (CallFunction|StartWave :!label _label))
      (:1
        (CallFunction|SetWaveInfo 1)
        (goto _label))
      (:2
        (CallFunction|SetWaveInfo 1)
        (goto _label))
      (:3
        (CallFunction|SetWaveInfo 1)
        (goto _label))
      (:4
        (CallFunction|SetWaveInfo 1)
        (goto _label))
      (:5
        (bind _outactors_2 (Actor|GetAllActorsOfClass "/Game/Blueprints/Enemies/Enemy.Enemy_C"))
        (for (_ _array_index) _outactors_2
          _)
        (if (not (Math|Conversions|ToBoolean(Integer) _array_index))
          (bind _returnvalue (UserInterface|CreateWidget "/Game/Blueprints/Widgets/WINSCREEN.WINSCREEN_C"))
          (UserInterface|Viewport|AddtoViewport _returnvalue 0))))))

(fn ConstructionScript)

(fn SetWaveInfo
  (params (Normal :type Integer) (Fast :type Integer) (Strong :type Integer))
  (|SetBy-RefVar (.number (Utilities|Struct|BreakenemyInfo (.Normal (Utilities|Struct|Breakwave (Variables|Default|GetwCurrent))))) Normal)
  (|SetBy-RefVar (.number (Utilities|Struct|BreakenemyInfo (.Fast (Utilities|Struct|Breakwave (Variables|Default|GetwCurrent))))) Fast)
  (|SetBy-RefVar (.number (Utilities|Struct|BreakenemyInfo (.Strong (Utilities|Struct|Breakwave (Variables|Default|GetwCurrent))))) Strong)
  (return))