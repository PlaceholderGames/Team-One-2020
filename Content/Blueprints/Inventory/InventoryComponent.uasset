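; Inventory component that holds a fixed number of item slots and shows or hides an inventory window.
; On BeginPlay it resizes the slot array to the configured count.
; Toggling creates the window with a reference to itself on the player controller's HUD canvas, or removes it if present.
; Adding handles only non-stackable items, passing them to CreateStack, which sets an array slot located by Find.
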(event EventBeginPlay
  (CallFunction|PrepareInventory))

(fn ToggleInventory
  (Utilities|IsValid 0
    (:Is%20Valid
      (Widget|RemovefromParent (Variables|Default|GetInventoryWindow))
      (Variables|Default|SetInventoryWindow 0))
    (:Is%20Not%20Valid
      (bind _returnvalue (UserInterface|CreateWidget "/Game/Blueprints/Inventory/InventoryUI/InventoryWindow.InventoryWindow_C" 0 self))
      (Variables|Default|SetInventoryWindow _returnvalue)
      (bind _asinv_player_controller (Utilities|Casting|CastToInvPlayerController (Game|GetPlayerController 0)))
      (bind _returnvalue_2 (Class|CanvasPanel|AddChildtoCanvas (Variables|/Game/Blueprints/Inventory/InventoryUI/InventoryHUD.InventoryHUD_C|GetHUDcanvas (Variables|/Game/Blueprints/Inventory/InvPlayerController.InvPlayerController_C|GetHUDwidget _asinv_player_controller)) (Variables|Default|GetInventoryWindow)))
      (Class|CanvasPanelSlot|SetAutoSize _returnvalue_2 true))))

(fn AddtoInventory
  (params (ContentToAdd :type Slot%20Structure%20Structure))
  (if (not (.isstackable (.itemstructure ContentToAdd)))
    (CallFunction|CreateStack ContentToAdd)
    (return true)))

(fn PrepareInventory
  (Utilities|Array|Resize (Variables|Default|GetInventory) (Variables|Default|GetNumberOfSlots)))

(fn CreateStack
  (params (ContentToAdd :type Slot%20Structure%20Structure))
  (bind _inventory (Variables|Default|GetInventory))
  (Utilities|Array|SetArrayElem :TargetArray _inventory :Index (Utilities|Array|FindItem :TargetArray _inventory)))