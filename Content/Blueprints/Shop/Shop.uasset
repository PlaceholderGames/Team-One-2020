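; Shop is a trigger-volume actor that opens the shop UI while the GeffPlaceholder character stands inside it.
; Entering TriggerBox creates the Shop widget, shows the cursor and switches to game-and-UI input; leaving removes the widget and restores game-only input.
; The menu sound plays on any actor's entry because it precedes the cast.
; An unconnected mouse-position clamp remains in the graph.
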(event OnComponentBeginOverlap(TriggerBox)
  (params (OverlappedComponent :type Primitive%20Component%20Object%20Reference) (OtherActor :type Actor%20Object%20Reference) (OtherComp :type Primitive%20Component%20Object%20Reference) (OtherBodyIndex :type Integer) (bFromSweep :type Boolean) (SweepResult :type Hit%20Result%20Structure%20%28by%20ref%29))
  (bind _returnvalue (Game|GetPlayerController 0))
  (Audio|PlaySoundatLocation "/Game/Sounds/offical_Sounds/SXF/Shop_Menu_SelectFinal.Shop_Menu_SelectFinal" (Transformation|GetActorLocation) "0, 0, 0" 1.0 1.0 0.0 0 0 0)
  (Utilities|Casting|CastToGeffPlaceholder OtherActor)
  (bind _returnvalue_2 (UserInterface|CreateWidget "/Game/Blueprints/Widgets/Shop.Shop_C"))
  (UserInterface|Viewport|AddtoViewport _returnvalue_2 0)
  (Variables|/Script/Engine.PlayerController|SetbShowMouseCursor _returnvalue true)
  (Input|SetInputModeGameandUI _returnvalue 0 "DoNotLock" false))

(event OnComponentEndOverlap(TriggerBox)
  (params (OverlappedComponent :type Primitive%20Component%20Object%20Reference) (OtherActor :type Actor%20Object%20Reference) (OtherComp :type Primitive%20Component%20Object%20Reference) (OtherBodyIndex :type Integer))
  (bind _returnvalue (Game|GetPlayerController 0))
  (Utilities|Casting|CastToGeffPlaceholder OtherActor)
  (Widget|RemovefromParent (stale OnComponentBeginOverlap(TriggerBox) _returnvalue_2))
  (Variables|/Script/Engine.PlayerController|SetbShowMouseCursor _returnvalue false)
  (Input|SetInputModeGameOnly _returnvalue))

(fn ConstructionScript)