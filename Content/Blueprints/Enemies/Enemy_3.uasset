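; Tower defense enemy that walks to the player base and damages it on contact.
; Every Tick it re-queries all actors of the target class and issues AI MoveTo to the first, or destroys itself when dead.
; Capsule overlaps with the base or a tower projectile deal its Damage to that actor and one point to itself.
; AnyDamage reduces health, which starts at MaxHealth, and destroys the enemy at zero.
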(event OnComponentBeginOverlap(CapsuleComponent)
  (params (OverlappedComponent :type Primitive%20Component%20Object%20Reference) (OtherActor :type Actor%20Object%20Reference) (OtherComp :type Primitive%20Component%20Object%20Reference) (OtherBodyIndex :type Integer) (bFromSweep :type Boolean) (SweepResult :type Hit%20Result%20Structure%20%28by%20ref%29))
  ;[1 1 1] Collision Checker
  (Variables|Default|SetColliding OtherActor)
  ;;[1 1 1] is it a base
  (if (== (Utilities|GetClass (Variables|Default|GetColliding)) "/Game/Blueprints/PlayerBase_Blueprint.PlayerBase_Blueprint_C")
    (CallFunction|BaseCollision (Variables|Default|GetColliding))
    (else
      ;;[1 1 1] is it a projectile
      (if (== (Utilities|GetClass (Variables|Default|GetColliding)) "/Game/Blueprints/Tower/TowerProjectile.TowerProjectile_C")
        (CallFunction|ProjectileCollision (Variables|Default|GetColliding))))))

(event Custom|MoveToTarget
  ;[1 1 1] Moves to Target
  (bind _outactors (Actor|GetAllActorsOfClass (Variables|Default|GetTarget)))
  (AI|AIMoveTo self "0, 0, 0" (Utilities|Array|Get(acopy) _outactors) 5.0 false))

(event Custom|BaseCollision
  (params (Base :type Actor%20Object%20Reference))
  ;[1 1 1] Collisions with the player base
  (Game|Damage|ApplyDamage Base (Variables|Default|GetDamage) 0 0)
  (Game|Damage|ApplyDamage self 1.0 0 0))

(event Custom|ProjectileCollision
  (params (Projectile :type Actor%20Object%20Reference))
  ;[1 1 1] Receiving damage from projectile
  (Game|Damage|ApplyDamage Projectile (Variables|Default|GetDamage) 0 0)
  (Game|Damage|ApplyDamage self 1.0 0 0))

(event EventTick
  (params (DeltaSeconds :type Float%20%28single-precision%29))
  ;[1 1 1] GameTick
  (bind _hashealth (CallFunction|IsAlive))
  (if _hashealth
    (CallFunction|MovetoTarget)
    (else
      (Actor|DestroyActor))))

(event Game|Damage|EventAnyDamage
  (params (Damage :type Float%20%28single-precision%29) (DamageType :type Damage%20Type%20Object%20Reference) (InstigatedBy :type Controller%20Object%20Reference) (DamageCauser :type Actor%20Object%20Reference))
  ;[1 1 1] Taking Damage
  (Variables|Default|SetCurrentHealth (- (Variables|Default|GetCurrentHealth) Damage))
  (if (<= (Variables|Default|GetCurrentHealth) 0.0)
    (Actor|DestroyActor)))

(fn ConstructionScript
  (Variables|Default|SetCurrentHealth (Variables|Default|GetMaxHealth))
  (CallFunction|SetTargetAny "/Game/Blueprints/PlayerBase_Blueprint.PlayerBase_Blueprint_C"))

(fn IsAlive
  (return (> (Variables|Default|GetCurrentHealth) 0.0)))

(fn SetTargetAny
  (params (TargetClass :type Actor%20Class%20Reference))
  (Variables|Default|SetTarget TargetClass))