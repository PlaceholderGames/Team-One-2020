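; Inventory component that holds a slot array and shows or hides the player's inventory window.
; On BeginPlay it resizes the array to NumberOfSlots.
; ToggleInventory adds a widget bound to the component to the MyPlayerController HUD canvas, or removes it, switching the mouse cursor.
; AddToInventory writes non-stackable items into the first empty slot, found by matching a zero-quantity struct; stackable items are not yet handled.
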(event EventBeginPlay
  (CallFunction|PrepareInventory))

(fn ToggleInventory
  ;[1 1 1] For creating the inventory on the screen
  (Variables|Default|GetInventoryWindow
    (:then
      (Widget|RemovefromParent (Variables|Default|GetInventoryWindow))
      (Variables|Default|SetInventoryWindow 0)
      (Variables|/Script/Engine.PlayerController|SetbShowMouseCursor (Game|GetPlayerController 0) false))
    (:else
      (bind _returnvalue (UserInterface|CreateWidget "/Game/Blueprints/InventorySystem/InventoryUI/InventoryWindow.InventoryWindow_C" 0 self))
      (Variables|Default|SetInventoryWindow _returnvalue)
      (bind _asmy_player_controller (Utilities|Casting|CastToMyPlayerController (Game|GetPlayerController 0)))
      (bind _returnvalue_2 (Class|CanvasPanel|AddChildtoCanvas (Variables|/Game/Blueprints/InventorySystem/InventoryUI/InventoryHUD.InventoryHUD_C|GetHudCanvas (Variables|/Game/Blueprints/InventorySystem/MyPlayerController.MyPlayerController_C|GetHUD%20Widget _asmy_player_controller)) (Variables|Default|GetInventoryWindow)))
      (Class|CanvasPanelSlot|SetAutoSize _returnvalue_2 true)
      (Variables|/Script/Engine.PlayerController|SetbShowMouseCursor (Game|GetPlayerController 0) true))))

(fn AddtoInventory
  (params (ContentToAdd :type Slot%20Structure%20Structure))
  ;[1 1 1] Creates new stacks if needed
  (if (not (.isstackable (.itemstructure ContentToAdd)))
    (CallFunction|CreateStack ContentToAdd)
    (return true)))

(fn PrepareInventory
  (Utilities|Array|Resize (Variables|Default|GetInventory) (Variables|Default|GetNumberOfSlots)))

(fn CreateStack
  (params (ContentToAdd :type Slot%20Structure%20Structure))
  (bind _inventory (Variables|Default|GetInventory))
  (Utilities|Array|SetArrayElem _inventory (Utilities|Array|FindItem _inventory (Utilities|Struct|MakeSlotStructure "(Name_2_25A8CC80487FE9D21222D193B3051945=NSLOCTEXT(\"[61D7EF3242C4F940DE834486F6D57625]\", \"44D20083497EC2939FB534A9402F7D63\", \"None\"),IsStackable_5_B932294F43CEE2FE3E29D485DCB75587=True,MaxStackSize_8_C24D452947B9608CB7AFB99D19CEDD3C=0,Class_18_18DEFF0445E5D04497A996834338270D=None,IsConsumable_14_938929A344D1486B71D14FB1A651B7D3=False,Description_17_AE820B43435CD3BB3326718F89791C04=NSLOCTEXT(\"[61D7EF3242C4F940DE834486F6D57625]\", \"96C09311475EE76A4EC7C586AB1FE991\", \"None\"),Thumbnail_21_2D16947B4D3FBD45BA5617B367255A6A=None)")) ContentToAdd))