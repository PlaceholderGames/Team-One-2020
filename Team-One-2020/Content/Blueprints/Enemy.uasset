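; Enemy that walks toward a target point and damages the player's base on contact.
; A delayed loop from BeginPlay repeatedly issues AI Move To toward the first TargetPoint found in the level.
; Capsule overlap with PlayerBase_Blueprint applies Damage to the base and one point to itself.
; AnyDamage reduces health; at zero it calls EnemyKilled on the base reference from the overlap cast and destroys itself.
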(event OnComponentBeginOverlap(CapsuleComponent)
  (params (OverlappedComponent :type Primitive%20Component%20Object%20Reference) (OtherActor :type Actor%20Object%20Reference) (OtherComp :type Primitive%20Component%20Object%20Reference) (OtherBodyIndex :type Integer) (bFromSweep :type Boolean) (SweepResult :type Hit%20Result%20Structure%20%28by%20ref%29))
  ;[1 1 1] Dealing Damage
  (bind _asplayer_base_blueprint (Utilities|Casting|CastToPlayerBase_Blueprint OtherActor))
  (Game|Damage|ApplyDamage _asplayer_base_blueprint (Variables|Default|GetDamage) 0 0)
  (Game|Damage|ApplyDamage self 1.0 0 0))

(event EventBeginPlay
  ;[1 1 1] Pathfinding
  (Variables|Default|SetCurrentHealth (Variables|Default|GetMaxHealth))
  (Utilities|FlowControl|Delay 0.2)
  (bind _outactors (Actor|GetAllActorsOfClass "/Script/Engine.TargetPoint" :!label _label))
  (AI|AIMoveTo self "0, 0, 0" (Utilities|Array|Get(acopy) _outactors) 5.0 false
    (:then
      (Utilities|FlowControl|Delay 0.2)
      (goto _label))))

(event Game|Damage|EventAnyDamage
  (params (Damage :type Float%20%28single-precision%29) (DamageType :type Damage%20Type%20Object%20Reference) (InstigatedBy :type Controller%20Object%20Reference) (DamageCauser :type Actor%20Object%20Reference))
  ;[1 1 1] Taking Damage
  (Variables|Default|SetCurrentHealth (- (Variables|Default|GetCurrentHealth) Damage))
  (if (<= (Variables|Default|GetCurrentHealth) 0.0)
    (Default|EnemyKilled (stale OnComponentBeginOverlap(CapsuleComponent) _asplayer_base_blueprint))
    (Actor|DestroyActor)))

(fn ConstructionScript)